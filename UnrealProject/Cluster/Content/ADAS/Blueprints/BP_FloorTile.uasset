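; BP_FloorTile is a road tile for an endless-runner style floor that scrolls its Scene component along negative X in repeating five-second moves.
; When BP_Car overlaps its Box, it has RunGameMode add a tile, then after a short delay removes itself from GMI_Cluster and destroys itself.
; On BeginPlay, a data-source boolean from GMI_Cluster toggles visibility of Scene's children as an ADAS mode.
; GetAttachTransform exposes the AttachPoint transform.
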(event OnComponentBeginOverlap(Box)
  (params (OverlappedComponent :type Primitive%20Component%20Object%20Reference) (OtherActor :type Actor%20Object%20Reference) (OtherComp :type Primitive%20Component%20Object%20Reference) (OtherBodyIndex :type Integer) (bFromSweep :type Boolean) (SweepResult :type Hit%20Result%20Structure%20%28by%20ref%29))
  ;[1 1 1] Next floor create
  (Utilities|Casting|CastToBP_Car OtherActor)
  (bind _asrun_game_mode (Utilities|Casting|CastToRunGameMode (Game|GetGameMode)))
  (Default|AddFloorTile _asrun_game_mode false)
  (Utilities|FlowControl|Delay 2.0)
  (bind _asgmi_cluster (Utilities|Casting|CastToGMI_Cluster (Game|GetGameInstance)))
  (Default|RemoveFloor _asgmi_cluster self)
  (Actor|DestroyActor))

(event Custom|RoadMove
  (bind _scene (Variables|Default|GetScene))
  (bind _relativelocation (Variables|/Script/Engine.SceneComponent|GetRelativeLocation _scene))
  ;[1 1 1] RoadMove
  (Utilities|Time|SetTimerbyEvent (delegate Custom|RoadMove) 5.0 true)
  (Components|MoveComponentTo _scene (Math|Vector|MakeVector (- (.x _relativelocation) (Variables|Default|GetMoveDistance)) (.y _relativelocation) (.z _relativelocation)) "0, 0, 0" false false 5.0 false))

(event EventBeginPlay
  (bind _asgmi_cluster (Utilities|Casting|CastToGMI_Cluster (Game|GetGameInstance)))
  (bind _datasourceinstance (Default|GetDataSourceInstance _asgmi_cluster))
  (bind _value (Default|GetDataValueBool _datasourceinstance "NewEnumerator0"))
  (CallFunction|ChangeMode _value)
  (CallFunction|RoadMove))

(fn ConstructionScript)

(fn GetAttachTransform
  (return (Transformation|GetWorldTransform (Variables|Default|GetAttachPoint))))

(fn ChangeMode
  (params (isADAS? :type Boolean))
  (for _array_element (Components|GetChildrenComponents (Variables|Default|GetScene) true)
    (Rendering|SetVisibility _array_element isADAS? false)))