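; Car actor for a cluster display's ADAS view, registering itself with GMI_Cluster on BeginPlay.
; A timeline drives GradientY on a dynamic background material created in the construction script.
; ChangeMode plays an ActorSequence and the background leave transition when ADAS is false; its reverse branch is unwired.
; SetCharge sets visibility on two cubes, then immediately applies the inverse to the same pair.
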(event Custom|LeaveADAS_BG
  (bind _gradienty (Timeline|BGChangeAnimation PlayFromStart)
    (:Update
      (Rendering|Material|SetScalarParameterValue (Variables|Default|GetBgADASMaterial) "GradientY" _gradienty :!class /Script/Engine.MaterialInstanceDynamic))))

(event Custom|EnterADAS_BG
  (bind _gradienty (Timeline|BGChangeAnimation ReverseFromEnd)
    (:Update
      (Rendering|Material|SetScalarParameterValue (Variables|Default|GetBgADASMaterial) "GradientY" _gradienty :!class /Script/Engine.MaterialInstanceDynamic))))

(event EventTick
  (params (DeltaSeconds :type Float%20%28single-precision%29)))

(event EventBeginPlay
  (bind _asgmi_cluster (Utilities|Casting|CastToGMI_Cluster (Game|GetGameInstance)))
  (Default|StoreOwnCarInstance _asgmi_cluster self))

(fn ConstructionScript
  (bind _returnvalue (Rendering|Material|CreateDynamicMaterialInstance (Variables|Default|GetBg_ADAS) 0 "/Game/Bg/M_Bg_ADAS.M_Bg_ADAS" "None" :!class /Script/Engine.PrimitiveComponent))
  (bind _output_get (Variables|Default|SetBgADASMaterial _returnvalue))
  (Rendering|Material|SetScalarParameterValue _output_get "GradientY" 0.0 :!class /Script/Engine.MaterialInstanceDynamic))

(fn ChangeMode
  (params (ADAS? :type Boolean))
  (if (not ADAS?)
    (Sequencer|Player|Play (Variables|/Script/ActorSequence.ActorSequenceComponent|GetSequencePlayer (Variables|Default|GetActorSequence)) :!class /Script/MovieScene.MovieSceneSequencePlayer)
    (CallFunction|LeaveADASBG)))

(fn StartupChangeBg
  (CallFunction|LeaveADASBG))

(fn SetCharge
  (params (isCharge :type Boolean))
  (bind _returnvalue (not isCharge))
  (Utilities|FlowControl|Sequence
    (:then_0
      (Rendering|SetVisibility (Variables|Default|GetCube) isCharge isCharge))
    (:then_1
      (Rendering|SetVisibility (Variables|Default|GetCube) _returnvalue _returnvalue))))