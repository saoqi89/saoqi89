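; Game mode for the ADAS run scene that unhides the player pawn on BeginPlay and provides floor tile spawning.
; AddFloorTile spawns a BP_ADASRoad and a random FloorArray tile, then stores the tile in GMI_Cluster.
; Only with IsFirstInit set does the tile's attach transform become the next spawn point.
; The ten-tile startup loop and tile mode switch are disconnected, and SetPawnVisible ignores its Visible input.
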(event EventBeginPlay
  (CallFunction|SetPawnVisible true))

(fn ConstructionScript)

(fn AddFloorTile
  (params (isFirstInit :type Boolean))
  (Game|SpawnActorfromClass "/Game/ADAS/Materials/ADAS_车道线/BP_ADASRoad.BP_ADASRoad_C" (Variables|Default|GetSpawn%20Transform) "Undefined" 0 0)
  (bind _returnvalue (Game|SpawnActorfromClass (Utilities|Array|Get(acopy) (Variables|Default|GetFloorArray) (Math|Random|RandomIntegerinRange 0 5)) (Variables|Default|GetNextSpawnPoint) "Undefined" 0 0))
  (bind _asbp_floor_tile (Utilities|Casting|CastToBP_FloorTile _returnvalue))
  (bind _asgmi_cluster (Utilities|Casting|CastToGMI_Cluster (Game|GetGameInstance)))
  (Default|StoreFloor _asgmi_cluster _asbp_floor_tile)
  (if isFirstInit
    (bind _attachtransform (Default|GetAttachTransform _asbp_floor_tile))
    (Variables|Default|SetNextSpawnPoint _attachtransform)))

(fn SetPawnVisible
  (params (visible :type Boolean))
  (Rendering|SetActorHiddenInGame (Game|Player|GetPlayerPawn 0) false))