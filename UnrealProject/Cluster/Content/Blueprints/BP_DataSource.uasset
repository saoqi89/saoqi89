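; BP_DataSource is a data store actor that holds named integer and boolean values in two maps.
; On BeginPlay it registers itself with the GMI_Cluster game instance.
; Its setters only overwrite keys that already exist in the maps, so unknown names are silently ignored.
; Its getters return the stored value, or a fallback of -1 or false when the name is missing.
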(event EventBeginPlay
  (bind _asgmi_cluster (Utilities|Casting|CastToGMI_Cluster (Game|GetGameInstance)))
  (Default|StoreDataSourceInstance _asgmi_cluster self))

(event Collision|EventActorBeginOverlap
  (params (OtherActor :type Actor%20Object%20Reference)))

(event EventTick
  (params (DeltaSeconds :type Float%20%28single-precision%29)))

(fn ConstructionScript)

(fn SetDataValueInt
  (params (Name :type Enum_DataInt%20Enum :default "NewEnumerator8") (Value :type Integer))
  (bind _dataintmap (Variables|Default|GetDataIntMap))
  (if (.ReturnValue (Utilities|Map|Find _dataintmap Name))
    (Utilities|Map|Add _dataintmap Name Value)))

(fn GetDataValueInt
  (params (name :type Enum_DataInt%20Enum :default "NewEnumerator0"))
  (bind _dataintmap (Variables|Default|GetDataIntMap))
  (bind (_value _returnvalue) (Utilities|Map|Find _dataintmap name))
  (if _returnvalue
    (return _value)
    (else
      (return -1))))

(fn SetDataValueBool
  (params (Name :type Enum_DataBool%20Enum :default "NewEnumerator0") (Value :type Boolean))
  (bind _databoolmap (Variables|Default|GetDataBoolMap))
  (if (.ReturnValue (Utilities|Map|Find _databoolmap Name))
    (Utilities|Map|Add _databoolmap Name Value)))

(fn GetDataValueBool
  (params (DataName :type Enum_DataBool%20Enum :default "NewEnumerator0"))
  (bind _databoolmap (Variables|Default|GetDataBoolMap))
  (bind (_value _returnvalue) (Utilities|Map|Find _databoolmap DataName))
  (if _returnvalue
    (return _value)
    (else
      (return false))))