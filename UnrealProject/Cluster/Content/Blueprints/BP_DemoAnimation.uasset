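; Demo driver for a vehicle instrument cluster that feeds animated fake data to the HMI when the build define is Debug or Release.
; Init caches the main UMG, data source and own-car references from GMI_Cluster, then a startup self-check timeline sweeps speed, energy and telltales.
; When it finishes, parallel timelines drive vehicle data, telltales, music and progress bars, while timeline events toggle ADAS, charging and drive modes.
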(event EventBeginPlay
  (bind _datasourceobj (Variables|Default|GetDataSourceObj))
  (bind _datasourceobj_2 (Variables|Default|GetDataSourceObj))
  (bind _umgobj (Variables|Default|GetUMGObj))
  (bind _umgobj_2 (Variables|Default|GetUMGObj))
  (bind _datasourceobj_3 (Variables|Default|GetDataSourceObj))
  (bind _umgobj_3 (Variables|Default|GetUMGObj))
  (bind _umgobj_4 (Variables|Default|GetUMGObj))
  (bind _test_ (CallFunction|Init))
  (if _test_
    (CallFunction|RivotekLog "NewEnumerator0" "BP_DemoAnimation" "" "Test or None. Do not to play animation.")
    (else
      (Utilities|FlowControl|Sequence
        (:then_1
          ;[1 1 1] Startup self check animation. Loop
          (bind (_direction _tt _tt_hide _speed _energy) (Timeline|startup_self_check Play)
            (:Update
              (Default|ShowTT _umgobj_2 (Math|Float|Truncate _tt))
              (Default|HideTT _umgobj_2 (Math|Float|Truncate _tt_hide))
              (Default|SetDataValueInt _datasourceobj "NewEnumerator8" (Math|Float|Truncate _speed))
              (Default|SetDataValueInt _datasourceobj "NewEnumerator7" (Math|Float|Truncate _energy)))
            (:Finished
              (Utilities|FlowControl|Delay 1.0)
              (Utilities|FlowControl|Sequence
                (:then_0
                  ;[1 1 1] Startup TT animation. Loop
                  (bind (_direction_2 _vehiclespeed _musiccard _tt_2 _tthide _powernum) (Timeline|DemoAnimation_TT Play)
                    (:Update
                      (Default|SetDataValueInt _datasourceobj_3 "NewEnumerator0" (Math|Float|Truncate _vehiclespeed))
                      (Default|ShowTT _umgobj (Math|Float|Truncate _tt_2))
                      (Default|HideTT _umgobj (Math|Float|Truncate _tthide))
                      (Default|SetDataValueInt _datasourceobj_3 "NewEnumerator7" (Math|Float|Truncate _powernum)))))
                (:then_1
                  ;[1 1 1] Startup commoninfo animation. Loop.
                  (bind (_direction_3 _time _odo) (Timeline|DemoAnimation_CommonInfo Play)
                    (:Update
                      (Default|SetDataValueInt (Variables|Default|GetDataSourceObj) "NewEnumerator1" (Math|Float|Truncate _time))
                      (Default|SetDataValueInt (Variables|Default|GetDataSourceObj) "NewEnumerator2" (Math|Float|Truncate _odo)))))
                (:then_2
                  ;[1 1 1] ADAS Mode Change. Loop.
                  (Timeline|DemoAnimation_module_3 Play
                    (:changemode
                      (Default|ChangeMode (Variables|Default|GetOwnCar) (Variables|Default|GetisADASMode))
                      (Default|SetDataValueBool (Variables|Default|GetDataSourceObj) "NewEnumerator0" (Math|Boolean|NotEqual(Boolean) (Variables|Default|GetisADASMode) true))
                      (for _array_element (Variables|/Game/Instance/GMI_Cluster.GMI_Cluster_C|GetFloorMap (Variables|Default|GetGMI_ClusterObj))
                        (Default|ChangeMode _array_element (Math|Boolean|NotEqual(Boolean) (Variables|Default|GetisADASMode) true))
                        (if (Math|Boolean|NotEqual(Boolean) (Variables|Default|GetisADASMode) true)
                          (Default|EnterAdas _umgobj_4)
                          (else
                            (Default|LeaveAdas _umgobj_4))))
                      (Variables|Default|SetisADASMode (Math|Boolean|NotEqual(Boolean) (Variables|Default|GetisADASMode) true)))
                    (:changeChargeMode
                      (Default|SetCharge (Variables|Default|GetOwnCar) (Variables|Default|GetisChargeMode))
                      (bind _output_get (Variables|Default|SetisChargeMode (not (Variables|Default|GetisChargeMode))))
                      (Default|SetDataValueBool (Variables|Default|GetDataSourceObj) "NewEnumerator1" _output_get))
                    (:ChangeRunMode
                      ;;[1 1 1] CarRunMode
                      (if (Variables|Default|GetIsSportMode)
                        (Default|SportMode _umgobj_3)
                        (Variables|Default|SetIsSportMode false)
                        (CallFunction|RivotekLog "NewEnumerator0" "BP_DemoAnimation" "" "SportMode")
                        (elif (Variables|Default|GetIsEcoMode)
                          (Default|EcoMode _umgobj_3)
                          (Variables|Default|SetIsEcoMode false)
                          (CallFunction|RivotekLog "NewEnumerator0" "BP_DemoAnimation" "" "EcoMode")
                          (else
                            (Default|TripPlay _umgobj_3)
                            (Variables|Default|SetIsEcoMode true)
                            (Variables|Default|SetIsSportMode true)
                            (CallFunction|RivotekLog "NewEnumerator0" "BP_DemoAnimation" "" "TripPlay")))))))
                (:then_4
                  ;[1 1 1 1 30] Startup Music and progress animation.Loop
                  (bind _musictime (Timeline|MusicTime Play)
                    (:Update
                      (Default|SetDataValueInt (Variables|Default|GetDataSourceObj) "NewEnumerator8" (Math|Float|Truncate _musictime))
                      (Default|SetDataValueInt (Variables|Default|GetDataSourceObj) "NewEnumerator6" (Math|Float|Truncate (/ (Math|Conversions|ToFloat(Integer) (Math|Float|Truncate _musictime)) 2.61))))))
                (:then_5
                  ;[1 1 1] ProgressBar
                  (bind (_direction_4 _progressbar1 _progressbar2) (Timeline|时间轴_1 Play)
                    (:Update
                      (Default|SetDataValueInt _datasourceobj_2 "NewEnumerator5" (Math|Float|Truncate _progressbar1))
                      (Default|SetDataValueInt _datasourceobj_2 "NewEnumerator4" (Math|Float|Truncate _progressbar2)))))))))))))

(fn ConstructionScript)

(fn Init
  (bind _asgmi_cluster (Utilities|Casting|CastToGMI_Cluster (Game|GetGameInstance)))
  (bind _output_get (Variables|Default|SetGMI_ClusterObj _asgmi_cluster))
  (bind _newparam (Default|GetDefine _output_get))
  (switch Utilities|FlowControl|Switch|SwitchonEnum_Define _newparam
    (:NewEnumerator3
      _)
    (:NewEnumerator0
      (bind _maininfoumg (Default|GetMainInfoUMG (Variables|Default|GetGMI_ClusterObj) :!label _label))
      (Variables|Default|SetUMGObj _maininfoumg)
      (bind _datasourceinstance (Default|GetDataSourceInstance (Variables|Default|GetGMI_ClusterObj)))
      (Variables|Default|SetDataSourceObj _datasourceinstance)
      (bind _result (Default|GetOwnCarInstance (Variables|Default|GetGMI_ClusterObj)))
      (Variables|Default|SetOwnCar _result)
      (return false))
    (:NewEnumerator1
      (goto _label))
    (:NewEnumerator2
      _))
  (return true))