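; Test actor for controlling a Niagara effect, apparently smoke, and picking actors under the cursor.
; BeginPlay shows the mouse cursor and enables input, so a touch press runs a visibility trace from the deprojected cursor, draws it persistently and prints the hit actor.
; OpenNiagara sets a fixed "direction" vector on the Niagara component of a referenced object.
; Unconnected leftover nodes for color, direction and velocity strength never run.
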(event Custom|OpenNiagara
  (Niagara|SetNiagaraVariable(Vector3) (Variables|/Script/Niagara.NiagaraActor|GetNiagaraComponent (Variables|Default|GetNewVar_0)) "direction" "45.000000,0.000000,45.000000"))

(event EventBeginPlay
  (bind _returnvalue (Game|GetPlayerController 0))
  (Variables|/Script/Engine.PlayerController|SetbShowMouseCursor _returnvalue true)
  (Input|EnableInput _returnvalue))

(event Collision|EventActorBeginOverlap
  (params (OtherActor :type Actor%20Object%20Reference)))

(event EventTick
  (params (DeltaSeconds :type Float%20%28single-precision%29)))

(event Input|KeyboardEvents|2
  (params (Key :type Key%20Structure :default "None")))

(event Input|KeyboardEvents|Up
  (params (Key :type Key%20Structure :default "None")))

(event Input|MouseEvents|LeftMouseButton
  (params (Key :type Key%20Structure :default "None")))

(event Input|KeyboardEvents|Down
  (params (Key :type Key%20Structure :default "None")))

(event Input|KeyboardEvents|Left
  (params (Key :type Key%20Structure :default "None")))

(event Input|KeyboardEvents|Right
  (params (Key :type Key%20Structure :default "None")))

(event Input|KeyboardEvents|R
  (params (Key :type Key%20Structure :default "None")))

(event Input|TouchEvents|InputTouch
  (params (Location :type Vector) (FingerIndex :type ETouchIndex%20Enum))
  (bind _returnvalue (Game|GetPlayerController 0))
  (bind (_worldlocation _worlddirection) (Game|Player|ConvertMouseLocationToWorldSpace _returnvalue))
  (:Pressed
    (bind _outhit (Collision|LineTraceByChannel _worldlocation (+ _worldlocation (* _worlddirection 1000)) "TraceTypeQuery1" true 0 "Persistent"))
    (Development|PrintString (Utilities|GetDisplayName (.HitActor (Collision|BreakHitResult _outhit))))))

(fn ConstructionScript)