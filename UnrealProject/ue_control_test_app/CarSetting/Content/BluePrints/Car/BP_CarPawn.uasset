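; BP_CarPawn is a car pawn with throttle, handbrake, and animated doors, windows and wipers, exposed as events.
; It registers itself with BP_CarSettingInst on BeginPlay, then each Tick passes scaled engine rotation speed to that instance's floor object.
; Throttle press applies full input, while release plays a slowdown timeline that feeds throttle input.
; Timelines drive part variables, reversing to close doors and windows and looping for the main wiper.
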(event Custom|ThrottleUpCar
  (bind _vehiclemovement (Variables|Default|GetVehicleMovement))
  ;[1 1 1] Movement control
  (Utilities|FlowControl|Sequence
    (:then_0
      (bind _speed (Timeline|SpeedSlowDown Stop)
        (:Update
          (Class|WheeledVehicleMovementComponent|SetThrottleInput _vehiclemovement _speed))))
    (:then_1
      (Class|WheeledVehicleMovementComponent|SetThrottleInput _vehiclemovement 1.0))))

(event Custom|ThrottleUpCarRelease
  (bind _vehiclemovement (Variables|Default|GetVehicleMovement))
  ;[1 1 1] Movement control
  (if (> (Class|WheeledVehicleMovementComponent|GetEngineRotationSpeed _vehiclemovement) 0.0)
    (bind _speed (Timeline|SpeedSlowDown PlayFromStart)
      (:Update
        (Class|WheeledVehicleMovementComponent|SetThrottleInput _vehiclemovement _speed)))))

(event Custom|OpenWindowR
  (bind _windowrval (Timeline|TL_WindowR Play)
    (:Update
      (Variables|CarControl|SetWindowR _windowrval))))

(event Custom|CloseWindowR
  (bind _windowrval (Timeline|TL_WindowR Reverse)
    (:Update
      (Variables|CarControl|SetWindowR _windowrval))))

(event Custom|StartWiper
  (Components|Timeline|SetLooping (Variables|Default|GetTL_Wiper) true)
  (bind (_direction _wiperxval _wiperyval) (Timeline|TL_Wiper PlayFromStart)
    (:Update
      (Variables|CarControl|SetWiperX _wiperxval)
      (Variables|CarControl|SetWiperY _wiperyval))))

(event Custom|StopWiper
  (Utilities|FlowControl|Sequence
    (:then_0
      (Components|Timeline|SetLooping (Variables|Default|GetTL_Wiper) false))
    (:then_1
      (bind (_direction _wiperxval _wiperyval) (Timeline|TL_Wiper Stop)
        (:Update
          (Variables|CarControl|SetWiperX _wiperxval)
          (Variables|CarControl|SetWiperY _wiperyval))))
    (:then_2
      (Timeline|TL_Wiper Play))))

(event Custom|StartWiper2
  (Timeline|TL_Wiper2 Play))

(event Custom|StopWiper2
  (Timeline|TL_Wiper2 Reverse))

(event Custom|StartWiperZ
  (Timeline|TL_WiperZ Play
    (:Update
      (Variables|CarControl|SetWiperZ 0.0))))

(event Custom|StopWiperZ
  (Timeline|TL_WiperZ Reverse
    (:Update
      (Variables|CarControl|SetWiperZ 0.0))))

(event Custom|HandBrakeRelease
  ;[1 1 1] Movement control
  (Class|WheeledVehicleMovementComponent|SetHandbrakeInput (Variables|Default|GetVehicleMovement) false))

(event Custom|HandBrake
  ;[1 1 1] Movement control
  (Class|WheeledVehicleMovementComponent|SetHandbrakeInput (Variables|Default|GetVehicleMovement) true))

(event Custom|OpenDoorL
  (bind _doorlval (Timeline|TL_DoorL Play)
    (:Update
      (Variables|CarControl|SetDoorL _doorlval))))

(event Custom|CloseDoorL
  (bind _doorlval (Timeline|TL_DoorL Reverse)
    (:Update
      (Variables|CarControl|SetDoorL _doorlval))))

(event Custom|OpenDoorR
  (bind _doorrval (Timeline|TL_DoorR Play)
    (:Update
      (Variables|CarControl|SetDoorR _doorrval))))

(event Custom|CloseDoorR
  (bind _doorrval (Timeline|TL_DoorR Reverse)
    (:Update
      (Variables|CarControl|SetDoorR _doorrval))))

(event Custom|OpenWindowL
  (bind _windowlval (Timeline|TL_WindowL Play)
    (:Update
      (Variables|CarControl|SetWindowL _windowlval))))

(event Custom|CloseWindowL
  (bind _windowlval (Timeline|TL_WindowL Reverse)
    (:Update
      (Variables|CarControl|SetWindowL _windowlval))))

(event EventBeginPlay
  (bind _asbp_car_setting_inst (Utilities|Casting|CastToBP_CarSettingInst (Game|GetGameInstance)))
  (Default|SetCarInst _asbp_car_setting_inst self))

(event EventTick
  (params (DeltaSeconds :type Float%20%28single-precision%29))
  (bind _vehiclemovement (Variables|Default|GetVehicleMovement))
  (bind _returnvalue (Class|WheeledVehicleMovementComponent|GetEngineRotationSpeed _vehiclemovement))
  (if (>= _returnvalue 0.0)
    (bind _floor (Default|GetFloor (stale EventBeginPlay _asbp_car_setting_inst)))
    (Default|SetSpeed _floor (/ _returnvalue 4e+03))))

(fn ConstructionScript)