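; BP_Floor is a floor actor whose car line material animates to suggest movement at an adjustable speed.
; The construction script applies a dynamic instance of MI_CarLine to its static mesh.
; On BeginPlay it registers itself with BP_CarSettingInst, then plays a timeline at zero rate that drives the material's movement parameter.
; SetSpeed changes the timeline's play rate, controlling how fast the lines move.
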(event EventBeginPlay
  (bind _asbp_car_setting_inst (Utilities|Casting|CastToBP_CarSettingInst (Game|GetGameInstance)))
  (Default|SetFloor _asbp_car_setting_inst self)
  (CallFunction|SetSpeed 0.0)
  (bind _movements (Timeline|TimeLine Play)
    (:Update
      (Rendering|Material|SetScalarParameterValue (Variables|Default|GetCarLineMaterial) "movement" _movements :!class /Script/Engine.MaterialInstanceDynamic))))

(event Collision|EventActorBeginOverlap
  (params (OtherActor :type Actor%20Object%20Reference)))

(event EventTick
  (params (DeltaSeconds :type Float%20%28single-precision%29)))

(fn ConstructionScript
  (bind _staticmesh (Variables|Default|GetStaticMesh))
  (bind _returnvalue (Rendering|Material|CreateDynamicMaterialInstance _staticmesh 0 "/Game/Material/MI_CarLine.MI_CarLine" "MI_Carline_DynInst" :!class /Script/Engine.PrimitiveComponent))
  (Variables|Default|SetCarLineMaterial _returnvalue)
  (Rendering|Material|SetMaterial _staticmesh 0 _returnvalue))

(fn SetSpeed
  (params (Speed :type Float%20%28single-precision%29))
  (Components|Timeline|SetPlayRate (Variables|Default|GetTimeLine) Speed))