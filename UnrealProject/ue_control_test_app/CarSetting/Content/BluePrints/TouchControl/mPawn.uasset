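; mPawn is a touch-control pawn that zooms its camera by changing a clamped SpringArm length.
; The mouse wheel steps the length directly, while the pinch axis compares each value with the last and passes a scaled ratio delta, gated by IsActivePinch, to PinchZooming.
; A DoOnce resets the pinch baseline per gesture, and debug prints show the delta.
; One-finger drag-to-look logic using 1Touch is present but disconnected.
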(event Input|AxisEvents|InputAxisPinchZoon
  (params (AxisValue :type Float%20%28single-precision%29))
  (bind _isactivepinch_ (Variables|Default|GetIsActivePinch?))
  ;[1 1 1] Pinch
  (if (not (== AxisValue (Variables|Default|GetPinchValue)))
    (Math|Float|CompareFloat AxisValue (Variables|Default|GetPinchValue)
      (:>
        (CallFunction|PinchZooming (* (- (Math|Float|Clamp(Float) (/ (Variables|Default|GetPinchValue) AxisValue)) 1.0) _isactivepinch_))
        (Development|PrintString (Utilities|String|ToString(Float) (* (- (Math|Float|Clamp(Float) (/ (Variables|Default|GetPinchValue) AxisValue)) 1.0) _isactivepinch_))))
      (:<
        (CallFunction|PinchZooming (* _isactivepinch_ (- 1.0 (Math|Float|Clamp(Float) (/ AxisValue (Variables|Default|GetPinchValue))))))
        (Development|PrintString (Utilities|String|ToString(Float) (* _isactivepinch_ (- 1.0 (Math|Float|Clamp(Float) (/ AxisValue (Variables|Default|GetPinchValue)))))) true true "(R=1.000000,G=0.000000,B=0.000000,A=1.000000)")))
    (Variables|Default|SetPinchValue AxisValue)))

(event Input|MouseEvents|MouseWheelUp
  (params (Key :type Key%20Structure :default "None"))
  (bind _springarm (Variables|Default|GetSpringArm))
  (:Pressed
    (Variables|/Script/Engine.SpringArmComponent|SetTargetArmLength _springarm (Math|Float|Clamp(Float) (- (Variables|/Script/Engine.SpringArmComponent|GetTargetArmLength _springarm) 1e+01) 1e+01 5e+02))))

(event Input|MouseEvents|MouseWheelDown
  (params (Key :type Key%20Structure :default "None"))
  (bind _springarm (Variables|Default|GetSpringArm))
  (:Pressed
    (Variables|/Script/Engine.SpringArmComponent|SetTargetArmLength _springarm (Math|Float|Clamp(Float) (+ (Variables|/Script/Engine.SpringArmComponent|GetTargetArmLength _springarm) 1e+01) 1e+01 5e+02))))

(event Input|KeyboardEvents|GesturePinch
  (params (Key :type Key%20Structure :default "None"))
  ;[1 1 1] Pinch
  ;;[0 0 0] Reset pinch value
  (:Pressed
    (Utilities|FlowControl|DoOnce false :!label _label
      (:Completed
        (Variables|Default|SetPinchValue 1.0))))
  (:Released
    (goto _label Reset)))

(event Input|TouchEvents|InputTouch
  (params (Location :type Vector) (FingerIndex :type ETouchIndex%20Enum)))

(fn ConstructionScript)

(fn 1Touch
  (bind _returnvalue (Game|GetPlayerController 0))
  (bind (_locationx _locationy) (Class|PlayerController|GetInputTouchState _returnvalue "Touch1"))
  (return (Math|Vector2D|MakeVector2D _locationx _locationy)))

(fn PinchZooming
  (params (PinchValue :type Float%20%28single-precision%29))
  (bind _springarm (Variables|Default|GetSpringArm))
  (Variables|/Script/Engine.SpringArmComponent|SetTargetArmLength _springarm (Math|Float|Clamp(Float) (+ (Variables|/Script/Engine.SpringArmComponent|GetTargetArmLength _springarm) (* PinchValue 1e+02)) 1e+01 5e+02)))